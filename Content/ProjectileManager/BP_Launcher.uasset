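; BP_Launcher is a keyboard-driven test actor for firing projectiles through its ProjectileLauncher and inspecting the projectile manager.
; Tick yaws the actor while Z or X is held and, when constant firing is toggled on, fires after a short Delay for a repeating stream.
; Number and Tab keys trigger single shots, toggle constant fire, print manager debug status and switch global time dilation between normal, slow and paused.
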(event EventTick
  (params (DeltaSeconds :type Float%20%28single-precision%29))
  (bind _returnvalue (Transformation|GetActorRotation))
  (bind _returnvalue_2 (Transformation|GetActorRotation))
  (bind _returnvalue_3 (Game|GetPlayerController 0))
  (if (Game|Player|IsInputKeyDown _returnvalue_3 "Z")
    (Transformation|SetActorRotation (Math|Rotator|MakeRotator (.roll _returnvalue) (.pitch _returnvalue) (+ (.yaw _returnvalue) -1.0))))
  (if (Game|Player|IsInputKeyDown _returnvalue_3 "X")
    (Transformation|SetActorRotation (Math|Rotator|MakeRotator (.roll _returnvalue_2) (.pitch _returnvalue_2) (+ (.yaw _returnvalue_2) 1.0))))
  (if (Variables|Default|GetConstantFiringIsOn)
    (Utilities|FlowControl|Delay 0.05)
    (Class|ProjectileLauncher|FireProjectile (Variables|Default|GetProjectileLauncher))))

(event Input|KeyboardEvents|4
  (params (Key :type Key%20Structure :default "None"))
  (:Pressed
    (Class|ProjectileManager|DebugPrintStatus (Subsystems|GetProjectileManager))))

(event Input|KeyboardEvents|3
  (params (Key :type Key%20Structure :default "None"))
  (:Pressed
    (Variables|Default|SetConstantFiringIsOn (not (Variables|Default|GetConstantFiringIsOn)))))

(event Input|KeyboardEvents|7
  (params (Key :type Key%20Structure :default "None"))
  (:Pressed
    (Utilities|Time|SetGlobalTimeDilation 1.0)))

(event Input|KeyboardEvents|Tab
  (params (Key :type Key%20Structure :default "None"))
  (:Pressed
    (Class|ProjectileLauncher|FireProjectile (Variables|Default|GetProjectileLauncher))))

(event Input|KeyboardEvents|8
  (params (Key :type Key%20Structure :default "None"))
  (:Pressed
    (Utilities|Time|SetGlobalTimeDilation 0.1)))

(event Input|KeyboardEvents|9
  (params (Key :type Key%20Structure :default "None"))
  (:Pressed
    (Utilities|Time|SetGlobalTimeDilation 0.0)))

(fn ConstructionScript)