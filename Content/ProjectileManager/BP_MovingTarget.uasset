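; Moving target actor that slides side to side along its local axes, with no sweep for collision.
; Tick offsets it by MoveDirection and MoveSpeed, scaled by world delta time.
; A Delay inside Tick acts as a repeating ten-second timer, flipping MoveSwitch to alternate the direction between left and right.
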(event EventTick
  (params (DeltaSeconds :type Float%20%28single-precision%29))
  (Transformation|AddActorLocalOffset (* (Variables|Default|GetMoveDirection) (Variables|Default|GetMoveSpeed) (Utilities|Time|GetWorldDeltaSeconds)) false false)
  (Utilities|FlowControl|Delay 1e+01)
  (Variables|Default|SetMoveSwitch (not (Variables|Default|GetMoveSwitch)))
  (if (not (Variables|Default|GetMoveSwitch))
    (Variables|Default|SetMoveDirection (Class|KismetMathLibrary|VectorLeft))
    (else
      (Variables|Default|SetMoveDirection (Class|KismetMathLibrary|VectorRight)))))

(fn ConstructionScript)